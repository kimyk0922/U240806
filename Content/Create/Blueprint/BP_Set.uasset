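; BP_Set builds and updates a square grid of BP_Cube tiles, some of which are marked as road.
; Evt_Spawn uses nested loops to spawn the cubes at even spacing in X and Y.
; Evt_Road gathers every BP_Cube, sets its Road flag by membership in this Blueprint's Road array, then calls EvtMap on it.
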(event Custom|Evt_Road
  (bind _outactors (Actor|GetAllActorsOfClass "/Game/Create/Blueprint/BP_Cube.BP_Cube_C"))
  (for _array_element _outactors
    (Variables|/Game/Create/Blueprint/BP_Cube.BP_Cube_C|SetbRoad _array_element (!= (Utilities|Array|FindItem (Variables|Default|GetRoad) _array_element) -1))
    (Default|EvtMap _array_element)))

(event Custom|Evt_Spawn
  (for _index (range 0 7)
    (for _index_2 (range 0 7)
      (Game|SpawnActorfromClass "/Game/Create/Blueprint/BP_Cube.BP_Cube_C" (Math|Transform|MakeTransform (Math|Vector|MakeVector (Math|Conversions|ToFloat(Integer) (* _index 200)) (Math|Conversions|ToFloat(Integer) (* _index_2 200)) 0.0) "0, 0, 0" "1.000000,1.000000,1.000000") "Undefined" "MultiplyWithRoot" 0 0))))

(fn ConstructionScript)