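; BP_Cube is a map tile cube that animates its height and material when the map event fires, depending on whether it is a road.
; Evt_Map delays by 2D distance from the world origin, staggering cubes into an outward ripple.
; Non-road cubes pick a random target height, road cubes keep the current target, and each type sets its own MValue.
; The Move timeline lerps the mesh's relative Z, then stores the new height.
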(event Custom|Evt_Map
  (bind _staticmesh (Variables|Default|GetStaticMesh))
  (Utilities|FlowControl|Delay (/ (Math|Vector|Distance2D(Vector) (Transformation|GetActorLocation self) "0, 0, 0") 1e+03))
  (if (Variables|Default|GetbRoad)
    (Rendering|Material|SetScalarParameterValueonMaterials _staticmesh "MValue" 0.0)
    (bind _newtrack_0 (Timeline|Move PlayFromStart)
      (:Update
        (Transformation|SetRelativeLocation (Variables|Default|GetStaticMesh) (Math|Vector|MakeVector 0.0 0.0 (Math|Float|Lerp (Variables|Default|GetBefore) (Variables|Default|GetAfter) _newtrack_0)) false false))
      (:Finished
        (Variables|Default|SetBefore (Variables|Default|GetAfter))))
    (else
      (Rendering|Material|SetScalarParameterValueonMaterials _staticmesh "MValue" 1.0)
      (Variables|Default|SetAfter (Math|Random|RandomFloatinRange 0.0 5e+01))
      (Timeline|Move PlayFromStart))))

(fn ConstructionScript)