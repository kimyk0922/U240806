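; BP_Tree is a cube-based tree tile that animates into either a flat road state or a raised tree.
; Evt_Ani waits in proportion to the actor's 2D distance from world origin, staggering the animation outward, then branches on Road.
; Road flags the body material and clears the head mesh; otherwise a switch, fixed at its first case, sets a wood head and random height.
; A timeline lerps the body's Z from Before to that target.
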(event Custom|Evt_Ani
  (bind _treebody (Variables|Default|GetTreeBody))
  (bind _treehead (Variables|Default|GetTreeHead))
  (Utilities|FlowControl|Delay (* (Math|Vector|Distance2D(Vector) "0, 0, 0" (Transformation|GetActorLocation)) 5e-05))
  (if (Variables|Default|GetbRoad)
    (Rendering|Material|SetScalarParameterValueonMaterials _treebody "bRoad" 1.0)
    (Components|StaticMesh|SetStaticMesh _treehead 0)
    (Variables|Default|SetAfter 0.0)
    (bind _newtrack_0 (Timeline|Timeline PlayFromStart)
      (:Update
        (Transformation|SetRelativeLocation (Variables|Default|GetTreeBody) (Math|Vector|MakeVector 0.0 0.0 (Math|Float|Lerp (Variables|Default|GetBefore) (Variables|Default|GetAfter) _newtrack_0)) false false))
      (:Finished
        (Variables|Default|SetAfter (Variables|Default|GetAfter))))
    (else
      (Rendering|Material|SetScalarParameterValueonMaterials _treebody "None" 0.0)
      (switch int 0
        (:0
          (Components|StaticMesh|SetStaticMesh _treehead "/Game/Create/Mesh/Sm_cube_wood.Sm_cube_wood")
          (Variables|Default|SetAfter (Math|Random|RandomFloatinRange 5e+01 3e+02))
          (Timeline|Timeline PlayFromStart))
        (:1
          (Components|StaticMesh|SetStaticMesh _treehead 0 :!label _label))
        (:2
          (goto _label))))))

(fn ConstructionScript)