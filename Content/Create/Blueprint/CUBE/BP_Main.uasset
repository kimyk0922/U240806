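; BP_Main manages a grid of BP_Tree actors and switches them through a sequence of road layouts.
; Evt_Spawn lays out the square grid, though nothing in this file calls it.
; BeginPlay starts a looping timer for Evt_Road, which flags each tree by membership in the current STRoad entry and triggers its EvtAni.
; Each pass advances the layout index with no wrap or bounds check.
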(event Custom|Evt_Spawn
  (for _index (range 0 7)
    (for _index_2 (range 0 7)
      (Game|SpawnActorfromClass "/Game/Create/Blueprint/CUBE/BP_Tree.BP_Tree_C" (Math|Transform|MakeTransform (Math|Vector|MakeVector (Math|Conversions|ToFloat(Integer) (* _index 300)) (Math|Conversions|ToFloat(Integer) (* _index_2 300)) 0.0) "0, 0, 0" "1.000000,1.000000,1.000000") "Undefined" "MultiplyWithRoot" 0 0))))

(event Custom|Evt_Road
  (bind _value (Variables|Default|GetValue))
  (bind _outactors (Actor|GetAllActorsOfClass "/Game/Create/Blueprint/CUBE/BP_Tree.BP_Tree_C"))
  (for _array_element _outactors
    (Variables|/Game/Create/Blueprint/CUBE/BP_Tree.BP_Tree_C|SetbRoad _array_element (!= (Utilities|Array|FindItem (Utilities|Struct|BreakST_Road (Utilities|Array|Get(acopy) (Variables|Default|GetST_Road) _value)) _array_element) -1))
    (Default|EvtAni _array_element))
  (Math|Integer|IncrementInt _value))

(event EventBeginPlay
  (Utilities|Time|SetTimerbyEvent (delegate Custom|Evt_Road) 1e+02 true))

(fn ConstructionScript)