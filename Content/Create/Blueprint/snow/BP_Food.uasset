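; BP_Food is a food pickup that restores BP_Player health while the player overlaps its Box.
; On overlap it disables player input, plays a one-shot animation on the player mesh, then after a one-second delay restores the Animation Blueprint and input.
; An Eat flag set by begin and end overlap makes Tick increment Health every frame, so healing is frame-rate dependent and has no cap here.
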(event OnComponentBeginOverlap(Box)
  (params (OverlappedComponent :type Primitive%20Component%20Object%20Reference) (OtherActor :type Actor%20Object%20Reference) (OtherComp :type Primitive%20Component%20Object%20Reference) (OtherBodyIndex :type Integer) (bFromSweep :type Boolean) (SweepResult :type Hit%20Result%20Structure%20%28by%20ref%29))
  (bind _returnvalue (Game|GetPlayerController 0))
  (bind _returnvalue_2 (Game|Player|GetPlayerPawn 0))
  (bind _asbp_player (Utilities|Casting|CastToBP_Player OtherActor))
  (Variables|Default|SetbEat true)
  (Input|DisableInput _returnvalue_2 _returnvalue)
  (Components|Animation|PlayAnimation (Variables|/Script/Engine.Character|GetMesh _asbp_player) 0 false)
  (Utilities|FlowControl|Delay 1.0)
  (Components|Animation|SetAnimationMode (Variables|/Script/Engine.Character|GetMesh _asbp_player) "AnimationBlueprint" true)
  (Input|EnableInput _returnvalue_2 _returnvalue))

(event OnComponentEndOverlap(Box)
  (params (OverlappedComponent :type Primitive%20Component%20Object%20Reference) (OtherActor :type Actor%20Object%20Reference) (OtherComp :type Primitive%20Component%20Object%20Reference) (OtherBodyIndex :type Integer))
  (Variables|Default|SetbEat false))

(event EventTick
  (params (DeltaSeconds :type Float%20%28single-precision%29))
  (if (Variables|Default|GetbEat)
    (Math|Float|IncrementFloat (Variables|/Game/Create/GM/BP_Player.BP_Player_C|GetHealth (stale OnComponentBeginOverlap(Box) _asbp_player)))))

(fn ConstructionScript)