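; BP_Snow is a snow hazard with a Box trigger that drains the player's Health over time.
; A begin overlap casts player pawn 0 to BP_Player, without checking the overlapping actor, and starts a looping one-second timer that decrements Health.
; End overlap or Evt_Stop re-sets that timer as non-looping, so one last decrement still fires a second later.
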(event OnComponentBeginOverlap(Box)
  (params (OverlappedComponent :type Primitive%20Component%20Object%20Reference) (OtherActor :type Actor%20Object%20Reference) (OtherComp :type Primitive%20Component%20Object%20Reference) (OtherBodyIndex :type Integer) (bFromSweep :type Boolean) (SweepResult :type Hit%20Result%20Structure%20%28by%20ref%29))
  (bind _asbp_player (Utilities|Casting|CastToBP_Player (Game|Player|GetPlayerPawn 0)))
  (Variables|Default|SetLooping true)
  (Utilities|Time|SetTimerbyEvent (delegate Custom|Evt_Health) 1.0 (Variables|Default|GetLooping)))

(event OnComponentEndOverlap(Box)
  (params (OverlappedComponent :type Primitive%20Component%20Object%20Reference) (OtherActor :type Actor%20Object%20Reference) (OtherComp :type Primitive%20Component%20Object%20Reference) (OtherBodyIndex :type Integer))
  (Variables|Default|SetLooping false)
  (Utilities|Time|SetTimerbyEvent (delegate Custom|Evt_Health) 1.0 (Variables|Default|GetLooping)))

(event Custom|Evt_Health
  (Math|Float|DecrementFloat (Variables|/Game/Create/GM/BP_Player.BP_Player_C|GetHealth (stale OnComponentBeginOverlap(Box) _asbp_player))))

(event Custom|Evt_Stop
  (Variables|Default|SetLooping false)
  (Utilities|Time|SetTimerbyEvent (delegate Custom|Evt_Health) 1.0 (Variables|Default|GetLooping)))

(fn ConstructionScript)