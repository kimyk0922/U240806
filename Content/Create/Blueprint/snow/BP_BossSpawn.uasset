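; BP_BossSpawn is an actor that spawns a ring of BP_Boss actors and contains an unfinished completion check.
; Evt_Spawn destroys tracked bosses, then spawns Value new ones evenly spaced 500 units around itself by rotating a vector about Z.
; Tick, gated by DoOnce, sets Complete when no level BP_Boss is missing from the tracked array.
; Its branch is hard-wired true, so it calls the empty ending event and never resets.
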(event Custom|Evt_Spawn
  (bind _value (Variables|Default|GetValue))
  (for _array_element (Variables|Default|GetBoss)
    (Actor|DestroyActor _array_element))
  (Utilities|Array|Clear (Variables|Default|GetBoss))
  (for _index (range 1 _value)
    (bind _returnvalue (Game|SpawnActorfromClass "/Game/Create/GM/BP_Boss.BP_Boss_C" (Math|Transform|MakeTransform (+ (Transformation|GetActorLocation) (* (Math|Vector|RotateVectorAroundAxis "1.000000,0.000000,0.000000" (* _index (/ 360 _value)) "0.000000,0.000000,1.000000") 5e+02)) "0, 0, 0" "1.000000,1.000000,1.000000") "Undefined" "MultiplyWithRoot" 0 0))
    (Utilities|Array|Add (Variables|Default|GetBoss) _returnvalue)))

(event Custom|Evt_Ending)

(event EventTick
  (params (DeltaSeconds :type Float%20%28single-precision%29))
  (Utilities|FlowControl|DoOnce false :!label _label
    (:Completed
      (bind _outactors (Actor|GetAllActorsOfClass "/Game/Create/GM/BP_Boss.BP_Boss_C"))
      (for _array_element _outactors
        (Utilities|Array|Add (Variables|Default|GetbDeath) (== (Utilities|Array|FindItem (Variables|Default|GetBoss) _array_element) -1)))
      (Variables|Default|SetComplete (== (Utilities|Array|FindItem (Variables|Default|GetbDeath) true) -1))
      (if true
        (CallFunction|EvtEnding)
        (else
          (Utilities|Array|Clear (Variables|Default|GetbDeath))
          (goto _label Reset))))))

(fn ConstructionScript)